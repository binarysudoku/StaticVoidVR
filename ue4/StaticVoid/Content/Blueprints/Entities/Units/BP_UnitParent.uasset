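; Parent Blueprint for units, providing a Move function that steers the actor toward TargetLocation until it is within a small tolerance.
; Speed interpolates toward MaxSpeed when far away and toward zero when close, driving a swept local offset along the world-space direction, unscaled by delta time.
; Rotation optionally interpolates toward a supplied target.
; Event graph and construction script are empty; Move prints current speed each call.
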(event EventBeginPlay)

(event Collision|EventActorBeginOverlap
  (params (OtherActor :type Actor%20Object%20Reference)))

(event EventTick
  (params (DeltaSeconds :type Float%20%28single-precision%29)))

(fn ConstructionScript)

(fn Move
  (params (TargetRelativeRotation :type Rotator) (DeltaTime :type Float%20%28single-precision%29) (OrientWhileMoving :type Boolean))
  (bind _returnvalue (Transformation|GetActorLocation))
  (bind _targetlocation (Variables|Default|GetTargetLocation))
  (Development|PrintString (Utilities|String|ToString(Float) (Variables|Default|GetCurrentSpeed)))
  ;[1 1 1] Interp Speed and Apply Movement
  (if (not (Math|Vector|Equal(Vector) _returnvalue _targetlocation 5.0))
    (if (>= (Math|Vector|VectorLength (- (Transformation|GetActorLocation) (Variables|Default|GetTargetLocation))) 2.5e+02)
      (Variables|Default|SetTarget%20Speed (Variables|Default|GetMaxSpeed))
      (else
        (Variables|Default|SetTarget%20Speed 0.0)))
    (Variables|Default|SetCurrentSpeed (Math|Interpolation|FInterpTo (Variables|Default|GetCurrentSpeed) (Variables|Default|GetTarget%20Speed) DeltaTime (Variables|Default|GetAcceleration)))
    (Transformation|AddActorLocalOffset (* (Class|KismetMathLibrary|GetDirectionVector _returnvalue _targetlocation) (Variables|Default|GetCurrentSpeed)) true false)
    ;[1 1 1] Interp Rotation
    (if OrientWhileMoving
      (Transformation|SetActorRotation (Math|Interpolation|RInterpTo (Transformation|GetActorRotation) TargetRelativeRotation DeltaTime (Variables|Default|GetRotationalAcceleration))))))