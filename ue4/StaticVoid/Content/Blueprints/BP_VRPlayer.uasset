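; VR player Blueprint that paints a selection volume and issues test movement targets to a ship.
; While Select is held, Tick spawns small BP_SelectSphere actors at CentreR every frame, as the trailing Delay gates nothing; releasing destroys them all.
; BeginPlay caches the first BP_TestShip and BP_TestTarget found.
; Two debug inputs set the ship's TargetLocation to the target actor's position or a hard-coded point.
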(event EventTick
  (params (DeltaSeconds :type Float%20%28single-precision%29))
  ;[1 1 1] Selection
  (if (Variables|Default|GetIsSelecting)
    (CallFunction|SpawnSelectVolume)
    (Utilities|FlowControl|Delay 0.05)))

(event EventBeginPlay
  (bind _outactors (Actor|GetAllActorsOfClass "/Game/Blueprints/Entities/Units/BP_TestShip.BP_TestShip_C"))
  (Variables|Default|SetTestShip (Utilities|Array|Get(acopy) _outactors))
  (bind _outactors_2 (Actor|GetAllActorsOfClass "/Game/Blueprints/Entities/Units/BP_TestTarget.BP_TestTarget_C"))
  (Variables|Default|SetTestTarget (Utilities|Array|Get(acopy) _outactors_2)))

(event Input|ActionEvents|InputActionTestMovement1
  (params (Key :type Key%20Structure :default "AnyKey"))
  (:Pressed
    (Development|PrintString "TestMovement1")
    (Variables|/Game/Blueprints/Entities/Units/BP_UnitParent.BP_UnitParent_C|SetTargetLocation (Variables|Default|GetTestShip) (Transformation|GetActorLocation (Variables|Default|GetTestTarget)))))

(event Input|ActionEvents|InputActionTestMovement2
  (params (Key :type Key%20Structure :default "AnyKey"))
  (:Pressed
    (Development|PrintString "Hello")
    (Variables|/Game/Blueprints/Entities/Units/BP_UnitParent.BP_UnitParent_C|SetTargetLocation (Variables|Default|GetTestShip) "-40.000000,-2.000000,0.000000")))

(event Input|ActionEvents|InputActionOrder
  (params (Key :type Key%20Structure :default "AnyKey")))

(event Input|ActionEvents|InputActionSelect
  (params (Key :type Key%20Structure :default "AnyKey"))
  (:Pressed
    (Variables|Default|SetIsSelecting true))
  (:Released
    (Variables|Default|SetIsSelecting false)
    (CallFunction|DeleteSelectVolume)))

(event Input|ActionEvents|InputActionMenuUp
  (params (Key :type Key%20Structure :default "AnyKey")))

(event Input|ActionEvents|InputActionMenuDown
  (params (Key :type Key%20Structure :default "AnyKey")))

(event Input|ActionEvents|InputActionMenuLeft
  (params (Key :type Key%20Structure :default "AnyKey")))

(event Input|ActionEvents|InputActionMenuRight
  (params (Key :type Key%20Structure :default "AnyKey")))

(fn ConstructionScript)

(fn SpawnSelectVolume
  (bind _returnvalue (Game|SpawnActorfromClass "/Game/Blueprints/Selection/BP_SelectSphere.BP_SelectSphere_C" (Math|Transform|MakeTransform (Transformation|GetWorldLocation (Variables|Default|GetCentre_R)) "0, 0,0.000000" "0.200000,0.200000,0.200000") "Undefined" 0 0))
  (Utilities|Array|Add (Variables|Default|GetSelectVolume) _returnvalue))

(fn DeleteSelectVolume
  (bind _selectvolume (Variables|Default|GetSelectVolume))
  (for _array_element _selectvolume
    (Actor|DestroyActor _array_element))
  (Utilities|Array|Clear _selectvolume))